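; BP_Target is a target actor that moves from BeginPlay and can take damage.
; A timeline adds its track value to the target mesh's local Y offset on each update, so movement accumulates frame by frame.
; The Damege event passes HP, damage value and target type to FLDamegeFunc, stores the returned HP, then destroys the actor without checking the result.
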(event `self.ReceiveBeginPlay`
  (`self.Move`))

(event `/Game/MY/Interface/BPI_Damage.Damege`
  (params (DamegeValue :type Integer) (TergetType :type "/Game/MY/Enum_Chalacter Enum" :default "NewEnumerator0"))
  (bind _newparam (`/Game/MY/FL.FLDamegeFunc` (`self.HP`) DamegeValue TergetType))
  (set `self.HP` _newparam)
  (`self.K2_DestroyActor`))

(event `Move`
  (bind (_direction _newtrack_1) (`Timeline|TimelineMove`)
    (:`Update`
      (`SceneComponent.K2_AddLocalOffset` (`self.TargetMesh`) (`KismetMathLibrary.MakeVector` 0.0 _newtrack_1) false false))))

(fn `UserConstructionScript`)